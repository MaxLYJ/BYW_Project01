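; Pickup actor that BP_Hand grabs through a short quick-time event.
; Trigger overlap calls ChangeSprite, then, for a hand, makes the pickup follow it each Tick.
; After a delay it shows the character's MyQTE, calls GetKeyDown and checks IsKeyDown after a randomized window.
; Success marks it grabbed and still following, failure returns it to its BeginPlay location, and both hide the QTE.
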(event OnComponentBeginOverlap(TriggerBox)
  (params (OverlappedComponent :type Primitive%20Component%20Object%20Reference) (OtherActor :type Actor%20Object%20Reference) (OtherComp :type Primitive%20Component%20Object%20Reference) (OtherBodyIndex :type Integer) (bFromSweep :type Boolean) (SweepResult :type Hit%20Result%20Structure%20%28by%20ref%29))
  (CallFunction|ChangeSprite)
  (bind _asbp_hand (Utilities|Casting|CastToBP_Hand OtherActor))
  (Variables|Default|SetAs%20BP%20Hand _asbp_hand)
  (Variables|Default|SetIsFollowMyHand true)
  (Utilities|FlowControl|Delay 0.5)
  (bind _returnvalue (Actor|GetActorOfClass "/Game/2DSideScrollerBP/Blueprints/2DSideScrollerCharacter.2DSideScrollerCharacter_C"))
  (Variables|/Script/UMG.Widget|SetVisibility (Variables|/Game/2DSideScrollerBP/Blueprints/2DSideScrollerCharacter.2DSideScrollerCharacter_C|GetmyQTE _returnvalue) "Visible")
  (Default|GetKeyDown _returnvalue)
  (Utilities|FlowControl|Delay (+ (/ (Math|Random|RandomFloat) 2.0) 0.2))
  (if (Variables|/Game/2DSideScrollerBP/Blueprints/2DSideScrollerCharacter.2DSideScrollerCharacter_C|GetIsKeyDown _returnvalue)
    (Variables|Default|SetIsGrabed true)
    (Variables|/Script/UMG.Widget|SetVisibility (Variables|/Game/2DSideScrollerBP/Blueprints/2DSideScrollerCharacter.2DSideScrollerCharacter_C|GetmyQTE _returnvalue) "Hidden")
    (else
      (Variables|Default|SetIsFollowMyHand false)
      (Transformation|SetActorLocation self (Variables|Default|GetMyOriginalLocation) false false)
      (Variables|/Script/UMG.Widget|SetVisibility (Variables|/Game/2DSideScrollerBP/Blueprints/2DSideScrollerCharacter.2DSideScrollerCharacter_C|GetmyQTE _returnvalue) "Hidden"))))

(event EventBeginPlay
  (Variables|Default|SetMyOriginalLocation (Transformation|GetActorLocation self))
  ;[1 1 1] Hide Texture
  (Rendering|Components|Sprite|SetSprite (Variables|Default|GetPaperSprite) "/Game/TexturesDemo01/T_hairband_Sprite.T_hairband_Sprite"))

(event Collision|EventActorBeginOverlap
  (params (OtherActor :type Actor%20Object%20Reference)))

(event EventTick
  (params (DeltaSeconds :type Float%20%28single-precision%29))
  (if (Variables|Default|GetIsFollowMyHand)
    (Transformation|SetActorLocation self (Transformation|GetActorLocation (Variables|Default|GetAs%20BP%20Hand)) false false)))

(fn ConstructionScript)

(fn ChangeSprite
  (params (NewSprite :type Paper%20Sprite%20Object%20Reference))
  (Rendering|Components|Sprite|SetSprite (Variables|Default|GetPaperSprite) NewSprite))