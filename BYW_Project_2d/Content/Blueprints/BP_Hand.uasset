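; BP_Hand is a flying hand in a 2D side-scroller that sweeps horizontally and can drop with a fetch sprite.
; Forces drive it, with tagged overlap volumes reversing it, sending it upward or resuming the sweep.
; HandDown starts the drop but is not called within this Blueprint.
; On returning to idle it opens YouWin if MyBattery is grabbed, otherwise it resets the sprite and briefly sets the player's IsDamagetime.
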(event EventBeginPlay
  (bind _returnvalue (Actor|GetActorOfClass "/Game/2DSideScrollerBP/Blueprints/2DSideScrollerCharacter.2DSideScrollerCharacter_C"))
  ;[1 1 1] Add initial force
  (Variables|Default|SetMyPlayer _returnvalue)
  (Pawn|Components|CharacterMovement|SetMovementMode (Variables|Character|GetCharacterMovement) "MOVE_Flying" 0)
  (Utilities|FlowControl|Delay 0.3)
  (Physics|AddForce (Variables|Character|GetCharacterMovement self) (Math|Vector|MakeVector (Variables|Default|GetMyForce) 0.0 0.0)))

(event Collision|EventActorBeginOverlap
  (params (OtherActor :type Actor%20Object%20Reference))
  (bind _self self)
  (bind _self_2 self)
  (bind _self_3 self)
  (bind _myplayer (Variables|Default|GetMyPlayer))
  (bind _charactermovement (Variables|Character|GetCharacterMovement _self))
  (bind _charactermovement_2 (Variables|Character|GetCharacterMovement _self_3))
  (bind _charactermovement_3 (Variables|Character|GetCharacterMovement _self_2))
  (Utilities|FlowControl|Sequence
    (:then_0
      ;[1 1 1] Trun Around
      (if (Actor|ActorHasTag OtherActor "TrunAround")
        (Development|PrintString "TurnAround")
        (Variables|/Script/Engine.MovementComponent|SetVelocity _charactermovement_3 "0, 0, 0")
        (Physics|AddForce _charactermovement_3 (Math|Vector|MakeVector (* (Variables|Default|GetMyForce) -1.0) 0.0 0.0))
        (Variables|Default|SetMyForce (* (Variables|Default|GetMyForce) -1.0))))
    (:then_1
      ;[1 1 1] Turn Up
      (if (Actor|ActorHasTag OtherActor "TurnUp")
        (Variables|/Script/Engine.MovementComponent|SetVelocity _charactermovement_2 "0, 0, 0")
        (Physics|AddForce _charactermovement_2 (Math|Vector|MakeVector 0.0 0.0 1e+07))))
    (:then_2
      ;[1 1 1] Back to idle
      (if (Actor|ActorHasTag OtherActor "BackToIdle")
        (Variables|/Script/Engine.MovementComponent|SetVelocity _charactermovement "0, 0, 0")
        (Physics|AddForce _charactermovement (Math|Vector|MakeVector (Variables|Default|GetMyForce) 0.0 0.0))
        (bind _asbp_pickup_actor (Utilities|Casting|CastToBP_PickupActor (Variables|Default|GetMyBattery)))
        (if (Variables|/Game/Blueprints/BP_PickupActor.BP_PickupActor_C|GetIsGrabed _asbp_pickup_actor)
          (Game|OpenLevel(byName) "YouWin")
          (else
            (Sprite|SetFlipbook (Variables|Default|GetSprite) "/Game/TexturesDemo01/T_hand.T_hand")
            (Variables|/Game/2DSideScrollerBP/Blueprints/2DSideScrollerCharacter.2DSideScrollerCharacter_C|SetIsDamagetime _myplayer true)
            (Utilities|FlowControl|Delay 1.0)
            (Variables|/Game/2DSideScrollerBP/Blueprints/2DSideScrollerCharacter.2DSideScrollerCharacter_C|SetIsDamagetime _myplayer false)))))))

(event EventTick
  (params (DeltaSeconds :type Float%20%28single-precision%29)))

(fn ConstructionScript)

(fn HandDown
  (bind _self self)
  (bind _charactermovement (Variables|Character|GetCharacterMovement _self))
  (Variables|/Script/Engine.MovementComponent|SetVelocity _charactermovement "0, 0, 0")
  (Physics|AddForce _charactermovement (Math|Vector|MakeVector 0.0 0.0 -1e+07))
  (Sprite|SetFlipbook (Variables|Default|GetSprite) "/Game/TexturesDemo01/T_handfetch4.T_handfetch4"))